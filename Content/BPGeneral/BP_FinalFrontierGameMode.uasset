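; BP_FinalFrontierGameMode is a game mode that sets up local players in levels whose name does not contain "menu".
; On BeginPlay it reads the player count from FinalFrontierGameInstance and creates local players until that count is reached.
; Each new player's auto-spawned pawn, if valid, is replaced by a possessed FirstPersonCharacter at one hardcoded location.
; PlayerStarts are gathered, but the random spawn-point helper is unused.
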(event `self.ReceiveBeginPlay`
  (bind _returnvalue (`GameplayStatics.GetCurrentLevelName` true))
  (if (== (`KismetStringLibrary.FindSubstring` _returnvalue "menu") -1)
    (bind _outactors (`GameplayStatics.GetAllActorsOfClass` "/Script/Engine.PlayerStart"))
    (set `self.SpawnPoints` _outactors)
    (bind _asfinal_frontier_game_instance (cast `FinalFrontierGameInstance` (`GameplayStatics.GetGameInstance`)))
    (bind _returnvalue_2 (`FinalFrontierGameInstance.getNumberOfPlayers` _asfinal_frontier_game_instance 0))
    (while (< (`self.CreatedPlayer`) _returnvalue_2)
      (bind _returnvalue_3 (`GameplayStatics.CreatePlayer` -1))
      (`/Engine/EditorBlueprintResources/StandardMacros.IncrementInt` (`self.CreatedPlayer`)
        (:`  `
          (`self.SpawnPlayer` _returnvalue_3))))))

(event `SpawnPlayer`
  (params (PlayerControler :type "PlayerController Object Reference"))
  (bind _returnvalue (`Controller.K2_GetPawn` PlayerControler))
  (`/Engine/EditorBlueprintResources/StandardMacros.IsValid` _returnvalue
    (:`Is Valid`
      (`self.K2_DestroyActor` _returnvalue)
      (bind _returnvalue_2 (`|SpawnActorFromClass` "/Game/FirstPersonCPP/Blueprints/FirstPersonCharacter.FirstPersonCharacter_C" (`KismetMathLibrary.MakeTransform` (-1793.756836 -1656.443359 332.000671)) "Undefined" "OverrideRootScale" null null))
      (`Controller.Possess` PlayerControler _returnvalue_2))))

(fn `UserConstructionScript`)